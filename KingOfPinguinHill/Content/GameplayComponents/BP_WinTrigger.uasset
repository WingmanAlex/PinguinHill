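; BP_WinTrigger is a kill-box actor that eliminates players and decides the match winner.
; On begin play it caches the BP_Camera and all ThirdPersonCharacters after a short delay.
; An overlapping character is removed from its list and the camera's, destroyed with a death sound, and player controllers blend to the shared camera.
; When one or fewer players remain, it writes the winner text to GI_cool and opens L_WinScreen.
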(event OnComponentBeginOverlap(KillBox)
  (params (OverlappedComponent :type Primitive%20Component%20Object%20Reference) (OtherActor :type Actor%20Object%20Reference) (OtherComp :type Primitive%20Component%20Object%20Reference) (OtherBodyIndex :type Integer) (bFromSweep :type Boolean) (SweepResult :type Hit%20Result%20Structure%20%28by%20ref%29))
  (if (== (Utilities|GetClass OtherActor) "/Game/ThirdPersonBP/Blueprints/ThirdPersonCharacter.ThirdPersonCharacter_C")
    (CallFunction|PlayerDead (.AsThird%20Person%20Character (Utilities|Casting|CastToThirdPersonCharacter OtherActor)))))

(event Custom|PlayerDead
  (params (player :type Third%20Person%20Character%20Object%20Reference))
  (bind _players (Variables|Default|GetPlayers))
  (Utilities|Array|RemoveItem _players player)
  (Utilities|Array|RemoveItem (Variables|/Game/GameplayComponents/BP_Camera.BP_Camera_C|GetPlayersRef (Variables|Default|GetCamera)) player)
  (Actor|DestroyActor player)
  (bind _outactors (Actor|GetAllActorsOfClass "/Script/Engine.PlayerController"))
  (Game|Player|SetViewTargetwithBlend _outactors (Variables|Default|GetCamera) 0.1 "VTBlend_Linear" 0.0 false)
  (Audio|PlaySound2D "/Game/Audio/die_Cue.die_Cue" 1.0 1.0 0.0 0 0)
  (if (<= (Utilities|Array|Length _players) 1)
    (Variables|/Game/MenuStuff/GI_cool.GI_cool_C|SetWinner (.AsGI%20Cool (Utilities|Casting|CastToGI_cool (Game|GetGameInstance))) (Utilities|Text|ToText(String) (Utilities|String|Append "Player " (Utilities|String|ToString(Integer) (Variables|/Game/ThirdPersonBP/Blueprints/ThirdPersonCharacter.ThirdPersonCharacter_C|GetPlayerIndex (Utilities|Array|Get(acopy) (Variables|Default|GetPlayers)))) " Wins!")))
    (Utilities|FlowControl|Delay 0.5)
    (Game|OpenLevel(byName) "L_WinScreen")))

(event EventBeginPlay
  (Utilities|FlowControl|Delay 0.2)
  (bind _returnvalue (Actor|GetActorOfClass "/Game/GameplayComponents/BP_Camera.BP_Camera_C"))
  (Variables|Default|SetCamera _returnvalue)
  (bind _outactors (Actor|GetAllActorsOfClass "/Game/ThirdPersonBP/Blueprints/ThirdPersonCharacter.ThirdPersonCharacter_C"))
  (Variables|Default|SetPlayers _outactors))

(fn ConstructionScript)