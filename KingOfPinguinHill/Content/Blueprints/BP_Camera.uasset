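; Shared multiplayer camera that keeps two to four players framed and becomes the view target for the player controllers.
; On BeginPlay it caches the players from BP_GameMode and starts a fast looping timer that drives updates instead of Tick.
; Each update picks a routine by player count, setting spring arm length to the clamped largest pairwise distance.
; It also interpolates the actor toward the players' average location for smooth following.
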(event Custom|UpdateCamera
  (switch int (Utilities|Array|Length (Variables|Default|GetPlayersRef))
    (:2
      (CallFunction|SetArmLenght2Players)
      (CallFunction|SetCameraPos2Players))
    (:3
      (CallFunction|SetArmLenght3Players)
      (CallFunction|SetCameraPos3Players))
    (:4
      (CallFunction|SetArmLenght4Players)
      (CallFunction|SetCameraPos4Players))))

(event EventBeginPlay
  (CallFunction|ClassSetup)
  (Utilities|Time|SetTimerbyFunctionName 0 "UpdateCamera" 0.001 true))

(fn ConstructionScript)

(fn ClassSetup
  (bind _asbp_game_mode (Utilities|Casting|CastToBP_GameMode (Game|GetGameMode)))
  (bind _output_get (Variables|Default|SetBP_GameMode _asbp_game_mode))
  (Variables|Default|SetPlayersRef (Variables|/Game/Blueprints/BP_GameMode.BP_GameMode_C|GetPlayers _output_get))
  (bind _outactors (Actor|GetAllActorsOfClass "/Script/Engine.PlayerController"))
  (Game|Player|SetViewTargetwithBlend _outactors self 0.0 "VTBlend_Linear" 0.0 false)
  (for (_array_element _array_index) (Variables|Default|GetPlayersRef)
    (switch int _array_index
      (:0
        (Variables|Default|SetPlayer1 _array_element))
      (:1
        (Variables|Default|SetPlayer2 _array_element))
      (:2
        (Variables|Default|SetPlayer3 _array_element))
      (:3
        (Variables|Default|SetPlayer4 _array_element)))))

(fn SetArmLenght4Players
  (bind _player1 (Variables|Default|GetPlayer1))
  (bind _player2 (Variables|Default|GetPlayer2))
  (bind _player3 (Variables|Default|GetPlayer3))
  (bind _player4 (Variables|Default|GetPlayer4))
  (Variables|/Script/Engine.SpringArmComponent|SetTargetArmLength (Variables|Default|GetSpringArm) (Math|Float|Clamp(Float) (.MaxValue (Math|Float|MaxOfFloatArray (Utilities|Array|MakeArray (Transformation|GetDistanceTo _player1 _player2) (Transformation|GetDistanceTo _player2 _player3) (Transformation|GetDistanceTo _player2 _player4) (Transformation|GetDistanceTo _player3 _player4) (Transformation|GetDistanceTo _player1 _player3) (Transformation|GetDistanceTo _player1 _player4)))) (Variables|Default|GetMinimumArmLenght) (Variables|Default|GetMaxArmLenght))))

(fn SetArmLenght3Players
  (bind _player1 (Variables|Default|GetPlayer1))
  (bind _player2 (Variables|Default|GetPlayer2))
  (bind _player3 (Variables|Default|GetPlayer3))
  (Variables|/Script/Engine.SpringArmComponent|SetTargetArmLength (Variables|Default|GetSpringArm) (Math|Float|Clamp(Float) (.MaxValue (Math|Float|MaxOfFloatArray (Utilities|Array|MakeArray (Transformation|GetDistanceTo _player1 _player2) (Transformation|GetDistanceTo _player2 _player3) (Transformation|GetDistanceTo _player1 _player3)))) (Variables|Default|GetMinimumArmLenght) (Variables|Default|GetMaxArmLenght))))

(fn SetArmLenght2Players
  (Variables|/Script/Engine.SpringArmComponent|SetTargetArmLength (Variables|Default|GetSpringArm) (Math|Float|Clamp(Float) (Transformation|GetDistanceTo (Variables|Default|GetPlayer1) (Variables|Default|GetPlayer2)) (Variables|Default|GetMinimumArmLenght) (Variables|Default|GetMaxArmLenght))))

(fn SetCameraPos4Players
  (Variables|Default|SetTargetPos (/ (+ (Transformation|GetActorLocation (Variables|Default|GetPlayer1)) (Transformation|GetActorLocation (Variables|Default|GetPlayer2)) (Transformation|GetActorLocation (Variables|Default|GetPlayer3)) (Transformation|GetActorLocation (Variables|Default|GetPlayer4))) (Math|Conversions|ToFloat(Integer) (Utilities|Array|Length (Variables|Default|GetPlayersRef)))))
  (Transformation|SetActorLocation (Math|Interpolation|VInterpTo (Variables|Default|GetPreviousPos) (Variables|Default|GetTargetPos) (Utilities|Time|GetWorldDeltaSeconds) (Variables|Default|GetInterpSpeed)) false false)
  (Variables|Default|SetPreviousPos (Transformation|GetActorLocation)))

(fn SetCameraPos3Players
  (Variables|Default|SetTargetPos (/ (+ (Transformation|GetActorLocation (Variables|Default|GetPlayer1)) (Transformation|GetActorLocation (Variables|Default|GetPlayer2)) (Transformation|GetActorLocation (Variables|Default|GetPlayer3))) (Math|Conversions|ToFloat(Integer) (Utilities|Array|Length (Variables|Default|GetPlayersRef)))))
  (Transformation|SetActorLocation (Math|Interpolation|VInterpTo (Variables|Default|GetPreviousPos) (Variables|Default|GetTargetPos) (Utilities|Time|GetWorldDeltaSeconds) (Variables|Default|GetInterpSpeed)) false false)
  (Variables|Default|SetPreviousPos (Transformation|GetActorLocation)))

(fn SetCameraPos2Players
  (Variables|Default|SetTargetPos (/ (+ (Transformation|GetActorLocation (Variables|Default|GetPlayer1)) (Transformation|GetActorLocation (Variables|Default|GetPlayer2))) (Math|Conversions|ToFloat(Integer) (Utilities|Array|Length (Variables|Default|GetPlayersRef)))))
  (Transformation|SetActorLocation (Math|Interpolation|VInterpTo (Variables|Default|GetPreviousPos) (Variables|Default|GetTargetPos) (Utilities|Time|GetWorldDeltaSeconds) (Variables|Default|GetInterpSpeed)) false false)
  (Variables|Default|SetPreviousPos (Transformation|GetActorLocation)))